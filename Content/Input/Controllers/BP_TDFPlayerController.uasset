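; BP_TDFPlayerController is a player controller holding debug hotkeys for exercising the TDF save subsystem.
; G saves to a fixed dev slot, H prints the number of existing save slots, and J creates a new test save.
; BeginPlay and the construction script are empty.
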(event EventBeginPlay)

(event Input|KeyboardEvents|G
  (params (Key :type Key%20Structure :default "None"))
  (:Pressed
    (Class|TDFSaveSubsystem|SaveGame (Subsystems|GetTDFSaveSubsystem) "DevSave" "Dev Save")))

(event Input|KeyboardEvents|H
  (params (Key :type Key%20Structure :default "None"))
  (:Pressed
    (Development|PrintString (Utilities|String|ToString(Integer) (Utilities|Array|Length (Class|TDFSaveSubsystem|GetSaveSlots (Subsystems|GetTDFSaveSubsystem)))))))

(event Input|KeyboardEvents|J
  (params (Key :type Key%20Structure :default "None"))
  (:Pressed
    (Class|TDFSaveSubsystem|CreateNewSave (Subsystems|GetTDFSaveSubsystem) "Test Save Two")))

(fn ConstructionScript)