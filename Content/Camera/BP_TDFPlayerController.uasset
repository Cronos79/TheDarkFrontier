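; BP_TDFPlayerController is the player controller that sets up the main HUD and building placement input.
; On BeginPlay it creates WBP_MainHud, adds it to the viewport, shows the cursor and switches to Game and UI input focused on the HUD.
; Left click, right click and R look up BP_BuildPlacementManager by class on each press to finish, cancel or rotate the placement ghost.
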(event EventBeginPlay
  (|CallParentFunction)
  (bind _returnvalue (UserInterface|CreateWidget "/Game/UI/WBP_MainHud.WBP_MainHud_C"))
  (Variables|Default|SetMainHud _returnvalue)
  (Input|SetInputModeGameandUI self (Variables|Default|GetMainHud) "DoNotLock" false false)
  (Variables|Default|SetbShowMouseCursor true)
  (UserInterface|Viewport|AddtoViewport (Variables|Default|GetMainHud) 0))

(event Input|MouseEvents|LeftMouseButton
  (params (Key :type Key%20Structure :default "None"))
  (:Pressed
    (bind _returnvalue (Actor|GetActorOfClass "/Game/Managers/BP_BuildPlacementManager.BP_BuildPlacementManager_C"))
    (Utilities|IsValid _returnvalue
      (:Is%20Valid
        (Class|BuildPlacementManager|FinishPlaceBuilding _returnvalue)))))

(event Input|MouseEvents|RightMouseButton
  (params (Key :type Key%20Structure :default "None"))
  (:Pressed
    (bind _returnvalue (Actor|GetActorOfClass "/Game/Managers/BP_BuildPlacementManager.BP_BuildPlacementManager_C"))
    (Utilities|IsValid _returnvalue
      (:Is%20Valid
        (Class|BuildPlacementManager|CancelPlacement _returnvalue)))))

(event Input|KeyboardEvents|R
  (params (Key :type Key%20Structure :default "None"))
  (:Pressed
    (bind _returnvalue (Actor|GetActorOfClass "/Game/Managers/BP_BuildPlacementManager.BP_BuildPlacementManager_C"))
    (Utilities|IsValid _returnvalue
      (:Is%20Valid
        (Class|BuildPlacementManager|RotatePlacementGhost _returnvalue)))))

(fn ConstructionScript)