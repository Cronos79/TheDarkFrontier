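; Player camera Blueprint that pans the view forward, back, left and right with hardcoded WASD key events.
; Each key's press and release sets a boolean, which Tick checks in a Sequence so multiple directions can apply in the same frame.
; Tick calls PanForward and PanRight, defined outside these graphs, passing MoveSpeed or NMoveSpeed for opposite directions, with no delta-time scaling in this graph.
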(event EventTick
  (params (DeltaSeconds :type Float%20%28single-precision%29))
  (bind _movespeed (Variables|Default|GetMoveSpeed))
  (bind _nmovespeed (Variables|Default|GetNMoveSpeed))
  (Utilities|FlowControl|Sequence
    (:then_0
      (if (Variables|Default|GetWPressed)
        (Class|TDFPlayerCamera|PanForward _movespeed)))
    (:then_1
      (if (Variables|Default|GetSPressed)
        (Class|TDFPlayerCamera|PanForward _nmovespeed)))
    (:then_2
      (if (Variables|Default|GetAPressed)
        (Class|TDFPlayerCamera|PanRight _nmovespeed)))
    (:then_3
      (if (Variables|Default|GetDPressed)
        (Class|TDFPlayerCamera|PanRight _movespeed)))))

(event Input|KeyboardEvents|W
  (params (Key :type Key%20Structure :default "None"))
  (:Pressed
    (Variables|Default|SetWPressed true))
  (:Released
    (Variables|Default|SetWPressed false)))

(event Input|KeyboardEvents|S
  (params (Key :type Key%20Structure :default "None"))
  (:Pressed
    (Variables|Default|SetSPressed true))
  (:Released
    (Variables|Default|SetSPressed false)))

(event Input|KeyboardEvents|A
  (params (Key :type Key%20Structure :default "None"))
  (:Pressed
    (Variables|Default|SetAPressed true))
  (:Released
    (Variables|Default|SetAPressed false)))

(event Input|KeyboardEvents|D
  (params (Key :type Key%20Structure :default "None"))
  (:Pressed
    (Variables|Default|SetDPressed true))
  (:Released
    (Variables|Default|SetDPressed false)))

(fn ConstructionScript)