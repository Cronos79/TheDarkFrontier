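; BP_StreamWater is a landscape actor that lays a stream water surface along an editable spline.
; The construction script adds one spline mesh per segment between consecutive StreamSpline points, using WaterMesh and matching local positions and tangents so the surface follows the curve.
; WaterWidthScale sets a uniform width and WaterZOffset shifts the surface vertically from the spline.
; The event graph holds no runtime logic.
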(event EventBeginPlay)

(event Collision|EventActorBeginOverlap
  (params (OtherActor :type Actor%20Object%20Reference)))

(event EventTick
  (params (DeltaSeconds :type Float%20%28single-precision%29)))

(fn ConstructionScript
  (bind _streamspline (Variables|Default|GetStreamSpline))
  (bind _streamspline_2 (Variables|Default|GetStreamSpline))
  (bind _waterwidthscale (Variables|Default|GetWaterWidthScale))
  (bind _waterzoffset (Variables|Default|GetWaterZOffset))
  (for _index (range 0 (- (Spline|GetNumberOfSplinePoints (Variables|Default|GetStreamSpline)) 2))
    (bind _returnvalue (AddComponent|AddSplineMeshComponent false (Math|Transform|MakeTransform "0, 0, 0" "0.000000,0.000000,0.000000" "1.000000,1.000000,1.000000")))
    (SplineMesh|SetStartScale _returnvalue (Math|Vector2D|MakeVector2D _waterwidthscale 1.0) true :!class /Script/Engine.SplineMeshComponent)
    (SplineMesh|SetEndScale _returnvalue (Math|Vector2D|MakeVector2D _waterwidthscale 1.0) true :!class /Script/Engine.SplineMeshComponent)
    (Transformation|AttachComponentToComponent _returnvalue (Variables|Default|GetStreamSpline) "None" "SnapToTarget" "SnapToTarget" "KeepRelative" true)
    (Components|StaticMesh|SetStaticMesh _returnvalue (Variables|Default|GetWaterMesh))
    (SplineMesh|SetStartandEnd _returnvalue (+ (Spline|GetLocationatSplinePoint _streamspline_2 _index "Local") (Math|Vector|MakeVector 0.0 0.0 _waterzoffset)) (Spline|GetTangentatSplinePoint _streamspline_2 _index "Local") (+ (Spline|GetLocationatSplinePoint _streamspline (+ _index 1) "Local") (Math|Vector|MakeVector 0.0 0.0 _waterzoffset)) (Spline|GetTangentatSplinePoint _streamspline (+ _index 1) "Local") true :!class /Script/Engine.SplineMeshComponent)))